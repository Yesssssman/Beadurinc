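; AI controller for Fighter enemies that runs BT_Fighter on possession and reacts to perception updates.
; A sensed Character tagged Player becomes the blackboard TargetActor, and that player's BeadurincPlayerController plays a busted sound and shows the fighter's boss bar.
; Any other Character update, lost sight or untagged, clears TargetActor and closes the boss bar on that character's controller, if it is a player's.
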(event OnTargetPerceptionUpdated(AIPerception)
  (params (Actor :type Actor%20Object%20Reference) (Stimulus :type AI%20Stimulus%20Structure))
  (bind _ascharacter (Utilities|Casting|CastToCharacter Actor))
  (if (and (Actor|ActorHasTag _ascharacter "Player") (.bSuccessfullySensed (Utilities|Struct|BreakAIStimulus Stimulus)))
    ;[0.15 0.15 0.15 0.5] On Perceive An Enemy
    (AI|Components|Blackboard|SetValueasObject (Variables|Default|GetBlackboard) (Variables|Default|GetTargetActor) _ascharacter)
    ;;[0.15 0.15 0.15 0.5] Send perceving alarm to player and add boss bar layer
    (bind _asbeadurinc_player_controller (Utilities|Casting|CastToBeadurincPlayerController (Pawn|GetController _ascharacter)))
    (Utilities|FlowControl|Sequence
      (:then_0
        (Class|BeadurincPlayerController|PlayLocalSound _asbeadurinc_player_controller "/Game/Sounds/SW_Busted.SW_Busted" 0.8))
      (:then_1
        (bind _asfighter_character (Utilities|Casting|CastToFighterCharacter (Pawn|GetControlledPawn)))
        (Class|BeadurincPlayerController|DisplayBossBar _asbeadurinc_player_controller _asfighter_character)))
    (else
      ;[0.15 0.15 0.15 0.5] No Enemies Detected
      (AI|Components|Blackboard|SetValueasObject (Variables|Default|GetBlackboard) (Variables|Default|GetTargetActor) 0)
      ;;[0.15 0.15 0.15 0.5] Send lost sensing event to remote player
      (bind _asbeadurinc_player_controller_2 (Utilities|Casting|CastToBeadurincPlayerController (Pawn|GetController _ascharacter)))
      (bind _asfighter_character_2 (Utilities|Casting|CastToFighterCharacter (Pawn|GetControlledPawn)))
      (Class|BeadurincPlayerController|CloseBossBar _asbeadurinc_player_controller_2 _asfighter_character_2))))

(event EventPossess
  (params (PossessedPawn :type Pawn%20Object%20Reference))
  (AI|RunBehaviorTree "/Game/AI/FIghter/BT_Fighter.BT_Fighter"))

(fn ConstructionScript)