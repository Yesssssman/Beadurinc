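; Player character Blueprint that tags itself as the player and shows a warning for dangerous attacks.
; AlertDangerAttacks picks a pierce or low-attack icon in the unblockable-alarm widget and plays an alert sound.
; A timeline scales the widget component, drives its material dissolve and turns it toward the follow camera, then hides it.
; The construction script makes the outfit mesh follow the main mesh through leader pose.
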(event EventBeginPlay
  (Variables|Default|SetTags (Utilities|Array|MakeArray "Player")))

(event EventAlertDangerAttacks
  (params (AttackType :type Gameplay%20Tag%20Structure%20%28by%20ref%29))
  (bind _widgetcomp (Variables|Default|GetWidgetComp))
  (Development|SetHiddeninGame _widgetcomp false true)
  (bind _aswbp_unblockable_alarm (Utilities|Casting|CastToWBP_Unblockable_Alarm (UserInterface|GetWidget _widgetcomp)))
  (Variables|/Game/Blueprints/Widgets/WBP_Unblockable_Alarm.WBP_Unblockable_Alarm_C|SetSelectedBrush _aswbp_unblockable_alarm (select (== AttackType "(TagName=\"AttackType.Pierce\")") (Variables|/Game/Blueprints/Widgets/WBP_Unblockable_Alarm.WBP_Unblockable_Alarm_C|GetPierceAttack _aswbp_unblockable_alarm) (Variables|/Game/Blueprints/Widgets/WBP_Unblockable_Alarm.WBP_Unblockable_Alarm_C|GetLowAttack _aswbp_unblockable_alarm)))
  (Audio|PlaySound2D "/Game/Sounds/SW_Busted.SW_Busted" 1.0 1.0 0.0 0 0)
  (bind (_direction _widgetscale _dissolvealpha) (Timeline|DissolveTimeline PlayFromStart)
    (:Update
      (Transformation|SetRelativeScale3D (Variables|Default|GetWidgetComp) (Math|Conversions|ToVector(Float) _widgetscale))
      (Rendering|Material|SetScalarParameterValue (UserInterface|GetMaterialInstance (Variables|Default|GetWidgetComp)) "DissolveAlpha" (Math|Float|Clamp(Float) _dissolvealpha) :!class /Script/Engine.MaterialInstanceDynamic)
      (Transformation|SetWorldRotation (Variables|Default|GetWidgetComp) (Math|Rotator|MakeRotationfromAxes (* (Math|Vector|GetForwardVector (Variables|Default|GetFollowCamera)) -1.0) "0, 0, 0" "0, 0, 0") false false))
    (:Finished
      (Development|SetHiddeninGame (Variables|Default|GetWidgetComp) true true))))

(fn ConstructionScript
  (Components|SkinnedMesh|SetLeaderPoseComponent (Variables|Default|GetOutfitMesh) (Variables|Character|GetMesh) false false))